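; BP_Tank is a tank Blueprint whose shown logic handles player aiming through a spring arm.
; Azimuth and elevation axes rotate the arm in yaw and pitch, scaled by frame delta time and per-axis sensitivity.
; The zoom axis adds to the arm length by a zoom speed, with no delta-time scaling or clamping.
; The construction script is empty.
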(event Input|AxisEvents|InputAxisAimAzimuth
  (params (AxisValue :type Float%20%28single-precision%29))
  (Transformation|AddRelativeRotation (Variables|Default|GetSpringArm) (Math|Rotator|MakeRotator 0.0 0.0 (* AxisValue (Utilities|Time|GetWorldDeltaSeconds) (Variables|Default|GetX%20Sensitivity) 1.0)) false false))

(event Input|AxisEvents|InputAxisAimElevation
  (params (AxisValue :type Float%20%28single-precision%29))
  (Transformation|AddRelativeRotation (Variables|Default|GetSpringArm) (Math|Rotator|MakeRotator 0.0 (* AxisValue (Utilities|Time|GetWorldDeltaSeconds) (Variables|Default|GetY%20Sensitivity)) 0.0) false false))

(event Input|AxisEvents|InputAxisAimZoom
  (params (AxisValue :type Float%20%28single-precision%29))
  (Variables|/Script/Engine.SpringArmComponent|SetTargetArmLength (Variables|Default|GetSpringArm) (+ (* AxisValue (Variables|Default|GetZoom%20Speed)) (Variables|/Script/Engine.SpringArmComponent|GetTargetArmLength (Variables|Default|GetSpringArm)))))

(fn ConstructionScript)