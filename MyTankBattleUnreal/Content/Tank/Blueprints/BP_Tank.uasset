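; Player tank Blueprint that provides orbit-camera aim controls and sets up the aiming component.
; On BeginPlay it hands the barrel mesh to the AimingComponent.
; Aim axes yaw the azimuth gimbal and pitch the spring arm separately, scaled by delta time and per-axis sensitivity.
; The zoom axis does nothing, as its spring arm length logic is disconnected.
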(event EventBeginPlay
  (Class|TankAimingComponent|SetBarrel (Variables|Default|GetAimingComponent) (Variables|Default|GetSM_Barrel)))

(event Input|AxisEvents|InputAxisAimAzimuth
  (params (AxisValue :type Float%20%28single-precision%29))
  (Transformation|AddLocalRotation (Variables|Default|GetAzimuthGimbal) (Math|Rotator|MakeRotator 0.0 0.0 (* AxisValue (Utilities|Time|GetWorldDeltaSeconds) (Variables|Default|GetX%20Sensitivity) 1.0)) false false))

(event Input|AxisEvents|InputAxisAimElevation
  (params (AxisValue :type Float%20%28single-precision%29))
  (Transformation|AddLocalRotation (Variables|Default|GetSpringArm) (Math|Rotator|MakeRotator 0.0 (* AxisValue (Utilities|Time|GetWorldDeltaSeconds) (Variables|Default|GetY%20Sensitivity)) 0.0) false false))

(event Input|AxisEvents|InputAxisAimZoom
  (params (AxisValue :type Float%20%28single-precision%29)))

(fn ConstructionScript)